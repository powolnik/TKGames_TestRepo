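; Interaction host that tracks registered interactionable objects, chooses which one is focused, and forwards Interact calls to it.
; Each Tick, it scores objects by the dot product between the ReferenceComponent's forward vector and the direction to their center, picking the best above a tolerance.
; SetFocused sends Focus and Unfocus calls as the selection changes, and unregistering the focused object clears it.
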(event `self.ReceiveTick`
  (params (DeltaSeconds :type "Float (single-precision)"))
  (`self.UpdateFocused`))

(event `RegisterInteractionable`
  (params (Object :type "/Game/Base/interactionable/BPI_Interactable Interface"))
  (`KismetArrayLibrary.Array_AddUnique` (`self.Interactionables`) Object)
  (`KismetSystemLibrary.PrintString` "ADDHello"))

(event `UnregisterInteractionable`
  (params (Object :type "/Game/Base/interactionable/BPI_Interactable Interface"))
  (`KismetArrayLibrary.Array_RemoveItem` (`self.Interactionables`) Object)
  (if (== (`KismetSystemLibrary.Conv_InterfaceToObject` Object) (`KismetSystemLibrary.Conv_InterfaceToObject` (`self.Focused`)))
    (`/Game/Base/interactionable/BPI_Interactable.Unfocus` (`self.Focused`))
    (set `self.Focused` null)
    (`KismetSystemLibrary.PrintString` "Unregister")))

(event `Interact`
  (`/Engine/EditorBlueprintResources/StandardMacros.IsValid` (`KismetSystemLibrary.Conv_InterfaceToObject` (`self.Focused`))
    (:`Is Valid`
      (`/Game/Base/interactionable/BPI_Interactable.Interact` (`self.Focused`)))))

(fn `SetFocused`
  (params (focused :type "/Game/Base/interactionable/BPI_Interactable Interface"))
  (locals (_local_focused :type "/Game/Base/interactionable/BPI_Interactable Interface"))
  (set `local._local_focused` focused)
  (`/Engine/EditorBlueprintResources/StandardMacros.IsValid` (`KismetSystemLibrary.Conv_InterfaceToObject` (`self.Focused`))
    (:`Is Valid`
      (`/Engine/EditorBlueprintResources/StandardMacros.IsValid` (`KismetSystemLibrary.Conv_InterfaceToObject` (`local._local_focused`))
        (:`Is Valid`
          (if (!= (`KismetSystemLibrary.Conv_InterfaceToObject` (`local._local_focused`)) (`KismetSystemLibrary.Conv_InterfaceToObject` (`self.Focused`)))
            (`/Game/Base/interactionable/BPI_Interactable.Unfocus` (`self.Focused`))
            (bind _output_get (set `self.Focused` (`local._local_focused`)))
            (`/Game/Base/interactionable/BPI_Interactable.Focus` _output_get)))
        (:`Is Not Valid`
          (`/Game/Base/interactionable/BPI_Interactable.Unfocus` (`self.Focused`))
          (set `self.Focused` (`local._local_focused`)))))
    (:`Is Not Valid`
      (`/Engine/EditorBlueprintResources/StandardMacros.IsValid` (`KismetSystemLibrary.Conv_InterfaceToObject` (`local._local_focused`))
        (:`Is Valid`
          (bind _output_get_2 (set `self.Focused` (`local._local_focused`)))
          (`/Game/Base/interactionable/BPI_Interactable.Focus` _output_get_2))))))

(fn `UpdateFocused`
  (locals (_dot :type "Float (double-precision)" :default 0.0) (_focused :type "/Game/Base/interactionable/BPI_Interactable Interface"))
  (bind _reference_component (`self.reference Component`))
  (if (> (`KismetArrayLibrary.Array_Length` (`self.Interactionables`)) 0)
    (for _array_element (`self.Interactionables`)
      (bind _center (message `/Game/Base/interactionable/BPI_Interactable.GetCenter` (`KismetSystemLibrary.Conv_InterfaceToObject` _array_element)))
      (bind _returnvalue (`KismetMathLibrary.Dot_VectorVector` (`KismetMathLibrary.Normal` (- _center (`SceneComponent.K2_GetComponentLocation` _reference_component))) (`SceneComponent.GetForwardVector` _reference_component)))
      (if (and (< (`self.Toleracne`) _returnvalue) (> _returnvalue (`local._dot`)))
        (set `local._dot` _returnvalue)
        (set `local._focused` _array_element)))
    (`/Engine/EditorBlueprintResources/StandardMacros.IsValid` (`KismetSystemLibrary.Conv_InterfaceToObject` (`local._focused`))
      (:`Is Valid`
        (`self.SetFocused` (`local._focused`)))
      (:`Is Not Valid`
        (`self.SetFocused` null)))))