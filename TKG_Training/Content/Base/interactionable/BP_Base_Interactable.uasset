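; Base interactable actor that registers with an overlapping actor's BP_InteractionHost while inside its sphere and, by default, destroys itself on Interact.
; Focus shows a widget, rotated each tick toward the CH_Player camera, and creates an outline; Unfocus reverses both.
; The outline is a runtime-spawned copy of the static mesh using a dynamic M_outline material with configurable color and scale.
; GetCenter exposes the mesh's center of mass.
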(event `self.ReceiveTick`
  (params (DeltaSeconds :type "Float (single-precision)"))
  (bind _asch_player (cast `/Game/Characters/Player/Blueprints/CH_Player` (`GameplayStatics.GetPlayerCharacter` 0)))
  (`SceneComponent.K2_SetWorldRotation` (`self.Widget`) (`KismetMathLibrary.FindLookAtRotation` (`SceneComponent.K2_GetComponentLocation` (`self.DefaultSceneRoot`)) (`SceneComponent.K2_GetComponentLocation` (`/Game/Characters/Player/Blueprints/CH_Player.Camera` _asch_player))) false false))

(event `self.Sphere.OnComponentBeginOverlap`
  (params (OverlappedComponent :type "PrimitiveComponent Object Reference") (OtherActor :type "Actor Object Reference") (OtherComp :type "PrimitiveComponent Object Reference") (OtherBodyIndex :type Integer) (bFromSweep :type Boolean) (SweepResult :type "HitResult Structure (by ref)"))
  (bind _returnvalue (`self.GetComponentByClass` OtherActor "/Game/Base/interactionable/BP_InteractionHost.BP_InteractionHost_C"))
  (`/Engine/EditorBlueprintResources/StandardMacros.IsValid` _returnvalue
    (:`Is Valid`
      (`/Game/Base/interactionable/BP_InteractionHost.RegisterInteractionable` _returnvalue self))))

(event `self.Sphere.OnComponentEndOverlap`
  (params (OverlappedComponent :type "PrimitiveComponent Object Reference") (OtherActor :type "Actor Object Reference") (OtherComp :type "PrimitiveComponent Object Reference") (OtherBodyIndex :type Integer))
  (bind _returnvalue (`self.GetComponentByClass` OtherActor "/Game/Base/interactionable/BP_InteractionHost.BP_InteractionHost_C"))
  (`/Engine/EditorBlueprintResources/StandardMacros.IsValid` _returnvalue
    (:`Is Valid`
      (`/Game/Base/interactionable/BP_InteractionHost.UnregisterInteractionable` _returnvalue self))))

(event `/Game/Base/interactionable/BPI_Interactable.Interact`
  (`self.K2_DestroyActor`))

(event `CreateOutline`
  (`self.Outline`
    (:`then`)
    (:`else`
      (bind _returnvalue (`AddComponent|NODE_AddStaticMeshComponent-0` :`RelativeTransform` (`SceneComponent.GetRelativeTransform` (`self.StaticMesh`))))
      (bind _output_get (set `self.Outline` _returnvalue))
      (`StaticMeshComponent.SetStaticMesh` _output_get (`StaticMeshComponent.StaticMesh` (`self.StaticMesh`)))
      (bind _returnvalue_2 (`PrimitiveComponent.CreateDynamicMaterialInstance` _output_get 0 "/Game/Base/interactionable/M_outline.M_outline" "None"))
      (`MaterialInstanceDynamic.SetVectorParameterValue` _returnvalue_2 "Color" (`self.OutlineColor`))
      (`MaterialInstanceDynamic.SetScalarParameterValue` _returnvalue_2 "Scale" (`self.OutlineScale`))
      (`KismetSystemLibrary.PrintString` "Hello"))))

(event `/Game/Base/interactionable/BPI_Interactable.Focus`
  (`SceneComponent.SetVisibility` (`self.Widget`) true false)
  (`self.CreateOutline`))

(event `/Game/Base/interactionable/BPI_Interactable.Unfocus`
  (`SceneComponent.SetVisibility` (`self.Widget`) false false)
  (`self.DestroyOutline`))

(event `DestroyOutline`
  (bind _outline (`self.Outline`)
    (:`then`
      (`ActorComponent.K2_DestroyComponent` _outline))
    (:`else`)))

(fn `GetCenter`
  (returns (Center :type "Vector Structure"))
  (return (`PrimitiveComponent.GetCenterOfMass` (`self.StaticMesh`) "None")))

(fn `UserConstructionScript`)